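; BP_Door_Locked is a locked door that opens only for a player holding a key.
; Any actor overlap adds a WBP_Interact prompt widget to the viewport, and end overlap removes the top-level widgets of that class.
; The OpenTheLockedDoor event checks that the player character overlaps BoxTrigger and has HasKey set on BP_Player, then instantly moves StaticDoor to a raised relative position.
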(event `self.ReceiveBeginPlay`)

(event `self.ReceiveActorBeginOverlap`
  (params (OtherActor :type "Actor Object Reference"))
  (bind _returnvalue (`|CreateWidget` "/Game/Boo/UI/WBP_Interact.WBP_Interact_C"))
  (`UserWidget.AddToViewport` _returnvalue 0))

(event `self.ReceiveActorEndOverlap`
  (params (OtherActor :type "Actor Object Reference"))
  (bind _foundwidgets (`WidgetBlueprintLibrary.GetAllWidgetsOfClass` "/Game/Boo/UI/WBP_Interact.WBP_Interact_C"))
  (`Widget.RemoveFromParent` _foundwidgets))

(event `Event OpenTheLockedDoor`
  (if (`PrimitiveComponent.IsOverlappingActor` (`self.BoxTrigger`) (`GameplayStatics.GetPlayerCharacter` 0))
    (bind _asbp_player (cast `/Game/FirstPersonCPP/Blueprints/BP_Player` (`GameplayStatics.GetPlayerCharacter` 0)))
    (if (`/Game/FirstPersonCPP/Blueprints/BP_Player.HasKey` _asbp_player)
      (`SceneComponent.K2_SetRelativeLocation` (`self.StaticDoor`) (0.0 0.0 200.0) false false))))

(fn `UserConstructionScript`)