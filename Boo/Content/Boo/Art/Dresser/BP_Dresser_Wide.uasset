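; A lockable wide dresser that holds a pearl necklace pickup, spawned and attached to its top drawer at BeginPlay.
; Looking at it within its overlap volume turns its meshes yellow and shows a widget with lock-state messages, which can be overridden.
; Interacting while locked inserts matching keys from the player's inventory and updates the prompt until all are in.
; Once unlocked, interacting plays the OpenDrawer timeline once and clears the highlight.
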(event `self.ReceiveBeginPlay`
  (bind _messagelineone_override_unlocked (`self.MessageLineOne_Override_Unlocked`))
  (bind _messagelinetwo_override_unlocked (`self.MessageLineTwo_Override_Unlocked`))
  (bind _messagelineone_override_locked (`self.MessageLineOne_Override_Locked`))
  (bind _messagelinetwo_override_locked (`self.MessageLineTwo_Override_Locked`))
  ;[1 1 1] Attach Loot/Pickup Mesh
  (bind _returnvalue (`|SpawnActorFromClass` "/Game/Boo/Art/BP_Pickup.BP_Pickup_C" (`KismetMathLibrary.MakeTransform` (0.0 0.0 0.0)) "Undefined" "OverrideRootScale"))
  (set `/Game/Boo/Art/BP_Pickup.Object` "PEARL NECKLACE" _returnvalue)
  (`SceneComponent.K2_AttachToComponent` (`/Game/Boo/Art/BP_Pickup.DefaultSceneRoot` _returnvalue) (`self.SM_Dresser_Wide_Drawer_Top`) "DrawerSocket" "KeepRelative" "KeepRelative" "KeepRelative" true)
  (if (`self.isLocked`)
    ;[1 1 1] Locked Messaging
    (if (`KismetStringLibrary.NotEqual_StrStr` _messagelineone_override_locked "DEFAULT")
      (set `self.MessageLineOne` _messagelineone_override_locked)
      (else
        (set `self.MessageLineOne` (`KismetStringLibrary.Concat_StrStr` "LOCKED " (`self.ObjectName`)))))
    (if (`KismetStringLibrary.NotEqual_StrStr` _messagelinetwo_override_locked "DEFAULT")
      (set `self.MessageLineTwo` _messagelinetwo_override_locked)
      (else
        (bind _fullyunlocked (`/Game/Boo/Art/BPFL_Interact.GetRemainingKeys` (`self.KeysToOpen`)))
        (set `self.MessageLineTwo` (`KismetStringLibrary.Concat_StrStr` " USE " (`KismetStringLibrary.JoinStringArray` _fullyunlocked "  ") " TO OPEN"))))
    (else
      ;[1 1 1] Unlocked Messaging
      (if (`KismetStringLibrary.NotEqual_StrStr` _messagelineone_override_unlocked "DEFAULT")
        (set `self.MessageLineOne` _messagelineone_override_unlocked)
        (else
          (set `self.MessageLineOne` (`KismetStringLibrary.Concat_StrStr` "UNLOCKED " (`self.ObjectName`)))))
      (if (`KismetStringLibrary.NotEqual_StrStr` _messagelinetwo_override_unlocked "DEFAULT")
        (set `self.MessageLineTwo` _messagelinetwo_override_unlocked)
        (else
          (set `self.MessageLineTwo` "CLICK TO OPEN"))))))

(event `self.ReceiveActorBeginOverlap`
  (params (OtherActor :type "Actor Object Reference"))
  ;[1 1 1] Tell the Player when they are in or out of the Check Volume
  (set `self.inRange` true))

(event `self.ReceiveActorEndOverlap`
  (params (OtherActor :type "Actor Object Reference"))
  ;[1 1 1] Tell the Player when they are in or out of the Check Volume
  (set `self.inRange` false)
  (`self.ResetMaterialsAndWidget`))

(event `/Game/Boo/Player/BPI_Player.StartLookingAt`
  ;[1 1 1] When the Object is Being Looked At, Change all Materials in the Mesh to Highlight It, and Create a Widget
  (if (`self.isOpened`)
    _
    (elif (`self.inRange`)
      (set `self.IsBeingLookedAt` true)
      (for _array_element (`self.K2_GetComponentsByClass` "/Script/Engine.StaticMeshComponent")
        (for _index (range (+ (`PrimitiveComponent.GetNumMaterials` _array_element) 1))
          (`PrimitiveComponent.SetMaterial` _array_element _index "/Game/Boo/MaterialLibrary/MI_Color_Yellow.MI_Color_Yellow")))
      (bind _returnvalue (`|CreateWidget` "/Game/Boo/UI/WBP_Interact.WBP_Interact_C"))
      (`/Game/Boo/UI/WBP_Interact.UpdateText` _returnvalue (`self.MessageLineOne`) (`self.MessageLineTwo`))
      (bind _foundwidgets (`WidgetBlueprintLibrary.GetAllWidgetsOfClass` "/Game/Boo/UI/WBP_Interact.WBP_Interact_C"))
      (if (not (> (`KismetArrayLibrary.Array_Length` _foundwidgets) 1))
        (`UserWidget.AddToViewport` _returnvalue 0)))))

(event `/Game/Boo/Player/BPI_Player.StopLookingAt`
  ;[1 1 1] Destroy the Widget and Reset the Materials when the Object is not being looked At
  (`self.ResetMaterialsAndWidget`))

(event `/Game/Boo/Player/BPI_Player.InteractObject`
  ;[1 1 1] Interact with Object
  (if (and (`self.IsBeingLookedAt`) (`self.inRange`))
    (if (`self.isLocked`)
      (`self.UnlockObject`)
      (elif (not (`self.isOpened`))
        (`TimelineComponent.SetPlayRate` (`self.Open Drawer`) (`self.PlayRate`))
        (`TimelineComponent.Play` (`self.Open Drawer`))
        (set `self.isOpened` true)
        (`self.ResetMaterialsAndWidget`)))))

(fn `ResetMaterialsAndWidget`
  (set `self.IsBeingLookedAt` false)
  (for _array_element (`self.K2_GetComponentsByClass` "/Script/Engine.StaticMeshComponent")
    (for _index (range (+ (`PrimitiveComponent.GetNumMaterials` _array_element) 1))
      (`PrimitiveComponent.SetMaterial` _array_element _index null)))
  (bind _foundwidgets (`WidgetBlueprintLibrary.GetAllWidgetsOfClass` "/Game/Boo/UI/WBP_Interact.WBP_Interact_C"))
  (`Widget.RemoveFromParent` _foundwidgets))

(fn `UnlockObject`
  (bind _messagelineone_override_unlocked (`self.MessageLineOne_Override_Unlocked`))
  (bind _messagelinetwo_override_unlocked (`self.MessageLineTwo_Override_Unlocked`))
  ;[1 1 1] Check Player Inventory for Required Keys
  (bind _asbp_player (cast `/Game/Boo/Player/BP_Player` (`GameplayStatics.GetPlayerCharacter` 0)))
  (bind _output (`/Game/Boo/Art/BPFL_Interact.GetRequiredKeysFromInventory` (`/Game/Boo/Player/BP_Player.Inventory` _asbp_player) (`self.KeysToOpen`)))
  (if (> (`KismetArrayLibrary.Array_Length` _output) 0)
    ;[1 1 1] Insert Required Keys from Player Inventory
    (bind _output_2 (`/Game/Boo/Art/BPFL_Interact.AddKeysToObject` _output (`self.KeysToOpen`)))
    (set `self.KeysToOpen` _output_2)
    (`/Game/Boo/Art/BPFL_Interact.RemoveKeysFromInventory` _output)
    ;[1 1 1] Check if all Keys are Inserted
    (bind _fullyunlocked (`/Game/Boo/Art/BPFL_Interact.AreAllKeysInserted` (`self.KeysToOpen`)))
    (if _fullyunlocked
      ;[1 1 1] If So Unlock Object
      (set `self.isLocked` false)
      (bind _foundwidgets (`WidgetBlueprintLibrary.GetAllWidgetsOfClass` "/Game/Boo/UI/WBP_Interact.WBP_Interact_C"))
      (if (`KismetStringLibrary.NotEqual_StrStr` _messagelineone_override_unlocked "DEFAULT")
        (set `self.MessageLineOne` _messagelineone_override_unlocked)
        (else
          (set `self.MessageLineOne` (`KismetStringLibrary.Concat_StrStr` "UNLOCKED " (`self.ObjectName`)))))
      (if (`KismetStringLibrary.NotEqual_StrStr` _messagelinetwo_override_unlocked "DEFAULT")
        (set `self.MessageLineTwo` _messagelinetwo_override_unlocked)
        (else
          (set `self.MessageLineTwo` "CLICK TO OPEN")))
      (`/Game/Boo/UI/WBP_Interact.UpdateText` _foundwidgets (`self.MessageLineOne`) (`self.MessageLineTwo`))
      (else
        ;[1 1 1] If Not, Show Keys Remaining
        (bind _foundwidgets_2 (`WidgetBlueprintLibrary.GetAllWidgetsOfClass` "/Game/Boo/UI/WBP_Interact.WBP_Interact_C"))
        (bind _fullyunlocked_2 (`/Game/Boo/Art/BPFL_Interact.GetRemainingKeys` (`self.KeysToOpen`)))
        (bind _output_get (set `self.MessageLineOne` (`KismetStringLibrary.Concat_StrStr` "LOCKED " (`self.ObjectName`))))
        (bind _output_get_2 (set `self.MessageLineTwo` (`KismetStringLibrary.Concat_StrStr` "YOU STILL NEED " (`KismetStringLibrary.JoinStringArray` _fullyunlocked_2) " TO OPEN")))
        (`/Game/Boo/UI/WBP_Interact.UpdateText` _foundwidgets_2 _output_get _output_get_2)))))

(fn `UserConstructionScript`)