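; BP_InteractiveDoor is a door that the player can open while standing in its trigger box.
; Any actor overlap adds a WBP_Interact widget to the viewport, then after a short delay removes top-level WBP_Overlay widgets rather than the one created.
; OpenTheDamnDoor snaps StaticDoor to a fixed raised position without sweep, provided the player character overlaps BoxTrigger.
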(event `self.ReceiveBeginPlay`)

(event `self.ReceiveActorBeginOverlap`
  (params (OtherActor :type "Actor Object Reference"))
  (bind _returnvalue (`|CreateWidget` "/Game/Boo/UI/WBP_Interact.WBP_Interact_C"))
  (`UserWidget.AddToViewport` _returnvalue 0)
  (`KismetSystemLibrary.Delay` 2.0)
  (bind _foundwidgets (`WidgetBlueprintLibrary.GetAllWidgetsOfClass` "/Game/Boo/UI/WBP_Overlay.WBP_Overlay_C"))
  (`Widget.RemoveFromParent` _foundwidgets))

(event `Event OpenTheDamnDoor`
  (if (`PrimitiveComponent.IsOverlappingActor` (`self.BoxTrigger`) (`GameplayStatics.GetPlayerCharacter` 0))
    (`SceneComponent.K2_SetRelativeLocation` (`self.StaticDoor`) (0.0 0.0 200.0) false false)))

(fn `UserConstructionScript`)