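; Searchable world object that the player can unlock, open and loot through look-at interaction.
; Overlap events track range; looking at it in range highlights every mesh material yellow and shows a prompt widget, restoring cached materials afterwards.
; InteractObject advances locked, opened, ready and empty flags, updating the prompt and showing a pickup widget.
; Keys and loot are strings in BP_Player's inventory, with "EMPTY" marking free slots.
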(event `self.ReceiveBeginPlay`
  ;[1 1 1] Read all Materials from Mesh, Create and Store in MaterialsList
  (bind _outputlist (`/Game/Boo/Art/BPFL_Interact.CreateMaterialList` (`self.StaticMesh`)))
  (set `self.MaterialsList` _outputlist)
  (if (`self.isLocked`)
    (set `self.WidgetString` (`KismetStringLibrary.Concat_StrStr` "LOCKED " (`self.ObjectName`) " USE " (`self.KeyToOpen`) " TO OPEN"))
    (else
      (set `self.isOpened` true)
      (set `self.WidgetString` (`KismetStringLibrary.Concat_StrStr` "UNLOCKED " (`self.ObjectName`) " CLICK TO OPEN")))))

(event `self.ReceiveActorBeginOverlap`
  (params (OtherActor :type "Actor Object Reference"))
  ;[1 1 1] Tell the Player when they are in or out of the Check Volume
  (bind _asbp_player (cast `/Game/Boo/Player/BP_Player` (`GameplayStatics.GetPlayerCharacter` 0)))
  (set `/Game/Boo/Player/BP_Player.numVolumesIsIn` (+ (`/Game/Boo/Player/BP_Player.numVolumesIsIn` _asbp_player) 1) _asbp_player)
  (set `self.inRange` true))

(event `self.ReceiveActorEndOverlap`
  (params (OtherActor :type "Actor Object Reference"))
  ;[1 1 1] Tell the Player when they are in or out of the Check Volume
  (bind _asbp_player (cast `/Game/Boo/Player/BP_Player` (`GameplayStatics.GetPlayerCharacter` 0)))
  (bind _output_get (set `/Game/Boo/Player/BP_Player.numVolumesIsIn` (- (`/Game/Boo/Player/BP_Player.numVolumesIsIn` _asbp_player) 1) _asbp_player))
  (set `self.inRange` false)
  (if (< 1 _output_get)
    (`self.ResetMaterialsAndWidget`)
    (goto _label :!via `Reset`)))

(event `/Game/Boo/Player/BPI_Player.StartLookingAt`
  ;[1 1 1] When the Object is Being Looked At, Change all Materials in the Mesh to Highlight It, and Create a Widget
  (if (`self.isEmpty`)
    _
    (elif (`self.inRange`)
      (set `self.IsBeingLookedAt` true)
      (for (_ _array_index) (`self.MaterialsList`)
        (`PrimitiveComponent.SetMaterial` (`self.StaticMesh`) _array_index "/Game/Boo/MaterialLibrary/MI_Color_Yellow.MI_Color_Yellow"))
      (bind _returnvalue (`|CreateWidget` "/Game/Boo/UI/WBP_Interact.WBP_Interact_C"))
      (`/Game/Boo/UI/WBP_Interact.UpdateText` _returnvalue (`self.WidgetString`) "")
      ;[1 1 1] Add The Widget to the Viewport Once
      (`/Engine/EditorBlueprintResources/StandardMacros.DoOnce` false :!label _label
        (:`Completed`
          (`UserWidget.AddToViewport` _returnvalue 0))))))

(event `/Game/Boo/Player/BPI_Player.StopLookingAt`
  ;[1 1 1] Destroy the Widget and Reset the Materials when the Object is not being looked At
  (`self.ResetMaterialsAndWidget`)
  (goto _label :!via `Reset`))

(event `/Game/Boo/Player/BPI_Player.InteractObject`
  ;[1 1 1] Object Interactions when Interacted
  (if (and (`self.IsBeingLookedAt`) (`self.inRange`))
    (if (`self.isLocked`)
      (`self.UnlockObject`)
      (elif (`self.isOpened`)
        (if (`KismetStringLibrary.EqualEqual_StrStr` (`self.Loot`) "EMPTY")
          (set `self.isEmpty` true)
          (set `self.isReady` false)
          (`self.ResetMaterialsAndWidget` :!label _label_2)
          (bind _returnvalue (`|CreateWidget` "/Game/Boo/UI/WBP_Pickup.WBP_Pickup_C" null (`self.Loot`)))
          (`UserWidget.AddToViewport` _returnvalue 0)
          (goto _label :!via `Reset`)
          (else
            (`self.OpenObject`)))
        (elif (`self.isReady`)
          (`self.CollectLoot`)
          (goto _label_2))))))

(fn `CollectLoot`
  (set `self.isReady` false)
  (set `self.isEmpty` true)
  (bind _asbp_player (cast `/Game/Boo/Player/BP_Player` (`GameplayStatics.GetPlayerCharacter` 0)))
  (bind _inventory (`/Game/Boo/Player/BP_Player.Inventory` _asbp_player))
  (`KismetArrayLibrary.Array_Set` _inventory (`KismetArrayLibrary.Array_Find` _inventory "EMPTY") (`self.Loot`)))

(fn `OpenObject`
  (if (`KismetStringLibrary.EqualEqual_StrStr` (`self.Loot`) "EMPTY")
    (set `self.isEmpty` true)
    (set `self.isReady` false)
    (`self.ResetMaterialsAndWidget`)
    (else
      (set `self.isReady` true)
      (set `self.isOpened` false)
      (bind _foundwidgets (`WidgetBlueprintLibrary.GetAllWidgetsOfClass` "/Game/Boo/UI/WBP_Interact.WBP_Interact_C"))
      (bind _output_get (set `self.WidgetString` (`KismetStringLibrary.Concat_StrStr` "OPEN " (`self.ObjectName`) " CLICK TO TAKE " (`self.Loot`))))
      (`/Game/Boo/UI/WBP_Interact.UpdateText` _foundwidgets _output_get ""))))

(fn `ResetMaterialsAndWidget`
  (set `self.IsBeingLookedAt` false)
  (for (_array_element _array_index) (`self.MaterialsList`)
    (`PrimitiveComponent.SetMaterial` (`self.StaticMesh`) _array_index _array_element))
  (bind _foundwidgets (`WidgetBlueprintLibrary.GetAllWidgetsOfClass` "/Game/Boo/UI/WBP_Interact.WBP_Interact_C"))
  (`Widget.RemoveFromParent` _foundwidgets))

(fn `UnlockObject`
  (bind _asbp_player (cast `/Game/Boo/Player/BP_Player` (`GameplayStatics.GetPlayerCharacter` 0)))
  (bind _inventory (`/Game/Boo/Player/BP_Player.Inventory` _asbp_player))
  (if (`KismetArrayLibrary.Array_Contains` _inventory (`self.KeyToOpen`))
    (set `self.isOpened` true)
    (set `self.isLocked` false)
    (`KismetArrayLibrary.Array_Set` _inventory (`KismetArrayLibrary.Array_Find` _inventory (`self.KeyToOpen`)) "EMPTY")
    (bind _foundwidgets (`WidgetBlueprintLibrary.GetAllWidgetsOfClass` "/Game/Boo/UI/WBP_Interact.WBP_Interact_C"))
    (bind _output_get (set `self.WidgetString` (`KismetStringLibrary.Concat_StrStr` "UNLOCKED " (`self.ObjectName`) " CLICK TO OPEN")))
    (`/Game/Boo/UI/WBP_Interact.UpdateText` _foundwidgets _output_get "")))

(fn `UserConstructionScript`)