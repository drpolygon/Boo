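; Temporary interactable door that can require several keys to unlock, accepting them incrementally from the player's inventory.
; While the player is in range and looking at it, the mesh turns yellow and WBP_Interact shows its lock state.
; Interacting moves matching keys into the door and updates the prompt with any still missing.
; Once unlocked, another interaction opens it by rescaling and moving the mesh, then restores its cached materials.
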(event `self.ReceiveBeginPlay`
  ;[1 1 1] Read Materials from Mesh, Create and Store in Materials List and Generate Widget String
  (set `self.keysRemaining` (`self.keysToOpen`))
  (bind _outputlist (`/Game/Boo/Art/BPFL_Interaction.CreateMaterialList` (`self.StaticDoor`)))
  (set `self.MaterialsList` _outputlist)
  (if (`self.isLocked`)
    (set `self.WidgetStringLineOne` (`KismetStringLibrary.Concat_StrStr` "LOCKED " (`self.DoorName`)))
    (`self.GetKeysRemaining`)
    (set `self.WidgetStringLineTwo` (`KismetStringLibrary.Concat_StrStr` " USE " (`KismetStringLibrary.JoinStringArray` (`self.keysToOpen`) "  ") " TO OPEN"))
    (else
      (set `self.WidgetStringLineOne` (`KismetStringLibrary.Concat_StrStr` "UNLOCKED " (`self.DoorName`)))
      (set `self.WidgetStringLineTwo` "CLICK TO OPEN"))))

(event `self.ReceiveActorBeginOverlap`
  (params (OtherActor :type "Actor Object Reference"))
  (bind _asbp_player (cast `/Game/Boo/Player/BP_Player` (`GameplayStatics.GetPlayerCharacter` 0)))
  (set `/Game/Boo/Player/BP_Player.isInCheckVolume` true _asbp_player)
  (set `self.inRange` true))

(event `self.ReceiveActorEndOverlap`
  (params (OtherActor :type "Actor Object Reference"))
  (bind _asbp_player (cast `/Game/Boo/Player/BP_Player` (`GameplayStatics.GetPlayerCharacter` 0)))
  (set `/Game/Boo/Player/BP_Player.isInCheckVolume` false _asbp_player)
  (set `self.inRange` false)
  (`self.ResetMaterialsAndWidget`)
  (goto _label :!via `Reset`))

(event `/Game/Boo/Player/BPI_Player.StartLookingAt`
  ;[1 1 1] When Door is Being Looked At, Change all Materials in the Mesh to Highlight It, and Create a Widget
  (if (`self.inRange`)
    (if (not (`self.isOpened`))
      (set `self.isBeingLookedAt` true)
      (for (_ _array_index) (`self.MaterialsList`)
        (`PrimitiveComponent.SetMaterial` (`self.StaticDoor`) _array_index "/Game/Boo/MaterialLibrary/MI_Color_Yellow.MI_Color_Yellow"))
      (bind _returnvalue (`|CreateWidget` "/Game/Boo/UI/WBP_Interact.WBP_Interact_C"))
      (`/Game/Boo/UI/WBP_Interact.UpdateText` _returnvalue (`self.WidgetStringLineOne`) (`self.WidgetStringLineTwo`))
      ;[1 1 1] Add Widget to Viewport Once
      (`/Engine/EditorBlueprintResources/StandardMacros.DoOnce` false :!label _label
        (:`Completed`
          (`UserWidget.AddToViewport` _returnvalue 0))))))

(event `/Game/Boo/Player/BPI_Player.StopLookingAt`
  ;[1 1 1] Destroy the Widget and Reset the Materials when the Object is not being looked At
  (`self.ResetMaterialsAndWidget`)
  (goto _label :!via `Reset`))

(event `/Game/Boo/Player/BPI_Player.InteractObject`
  (if (and (`self.isBeingLookedAt`) (`self.inRange`))
    (if (`self.isLocked`)
      (`self.UnlockDoor`)
      (elif (not (`self.isOpened`))
        (`self.OpenDoor`)
        (`self.ResetMaterialsAndWidget`)
        (goto _label :!via `Reset`)))))

(fn `GetKeysRemaining`
  (for _array_element (`self.keysToOpen`)
    (if (`KismetArrayLibrary.Array_Contains` (`self.keysInDoor`) _array_element)
      (`KismetArrayLibrary.Array_RemoveItem` (`self.keysRemaining`) _array_element)))
  (return))

(fn `OpenDoor`
  (bind _staticdoor (`self.StaticDoor`))
  (set `self.isOpened` true)
  (`SceneComponent.SetRelativeScale3D` _staticdoor (0.3 1.0 0.125))
  (`SceneComponent.K2_SetRelativeLocation` _staticdoor (-60.0 0.0 240.0) false false)
  (bind _foundwidgets (`WidgetBlueprintLibrary.GetAllWidgetsOfClass` "/Game/Boo/UI/WBP_Interact.WBP_Interact_C"))
  (`Widget.RemoveFromParent` _foundwidgets))

(fn `ResetMaterialsAndWidget`
  (set `self.isBeingLookedAt` false)
  (for (_array_element _array_index) (`self.MaterialsList`)
    (`PrimitiveComponent.SetMaterial` (`self.StaticDoor`) _array_index _array_element))
  (bind _foundwidgets (`WidgetBlueprintLibrary.GetAllWidgetsOfClass` "/Game/Boo/UI/WBP_Interact.WBP_Interact_C"))
  (`Widget.RemoveFromParent` _foundwidgets))

(fn `UnlockDoor`
  (bind _keysindoor (`self.keysInDoor`))
  (`self.GetKeysRemaining`)
  (bind _asbp_player (cast `/Game/Boo/Player/BP_Player` (`GameplayStatics.GetPlayerCharacter` 0)))
  ;[1 1 1] Check if Player Has Any Remaining Keys in Inventory
  (for _array_element (`self.keysRemaining`)
    (bind _inventory (`/Game/Boo/Player/BP_Player.Inventory` _asbp_player))
    ;[1 1 1] If so, remove keys from Inventory and Add to Door
    (if (`KismetArrayLibrary.Array_Contains` _inventory _array_element)
      (`KismetArrayLibrary.Array_Set` _inventory (`KismetArrayLibrary.Array_Find` _inventory _array_element) "EMPTY")
      (`KismetArrayLibrary.Array_Set` _keysindoor (`KismetArrayLibrary.Array_Find` _keysindoor "") _array_element)))
  ;[1 1 1] If there are no keys remaining...
  (`self.GetKeysRemaining`)
  (if (== (`KismetArrayLibrary.Array_Length` (`self.keysRemaining`)) 0)
    (set `self.isLocked` false)
    ;[1 1 1] Unlock The Door and Empty Player Inventory of Keys
    (for _ (`self.keysRemaining`)
      (`KismetArrayLibrary.Array_Set` _inventory (`KismetArrayLibrary.Array_Find` _inventory (`self.keyToOpen`)) "EMPTY")
      (bind _foundwidgets (`WidgetBlueprintLibrary.GetAllWidgetsOfClass` "/Game/Boo/UI/WBP_Interact.WBP_Interact_C" :!label _label))
      (bind _output_get (set `self.WidgetStringLineOne` (`KismetStringLibrary.Concat_StrStr` "UNLOCKED " (`self.DoorName`))))
      (`/Game/Boo/UI/WBP_Interact.UpdateText` _foundwidgets _output_get "CLICK TO OPEN"))
    (goto _label)
    (else
      ;[1 1 1] If Door Still Locked, Show Keys Remaining
      (bind _foundwidgets_2 (`WidgetBlueprintLibrary.GetAllWidgetsOfClass` "/Game/Boo/UI/WBP_Interact.WBP_Interact_C"))
      (bind _output_get_2 (set `self.WidgetStringLineOne` (`KismetStringLibrary.Concat_StrStr` "LOCKED " (`self.DoorName`))))
      (`/Game/Boo/UI/WBP_Interact.UpdateText` _foundwidgets_2 _output_get_2 (`KismetStringLibrary.Concat_StrStr` "YOU STILL NEED " (`KismetStringLibrary.JoinStringArray` (`self.keysRemaining`)) " TO OPEN")))))

(fn `UserConstructionScript`)