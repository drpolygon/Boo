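; Interactive treasure chest that the player unlocks with a named key, opens and loots.
; While the player overlaps its sphere, Tick traces from the camera, highlights the targeted chest and creates a WBP_Interact status prompt each frame.
; Unlock, open and loot events check range, highlight and chest state.
; Inventory is a string array using "EMPTY" slots: unlocking consumes the key, looting fills a free slot.
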(event `self.Sphere.OnComponentBeginOverlap`
  (params (OverlappedComponent :type "PrimitiveComponent Object Reference") (OtherActor :type "Actor Object Reference") (OtherComp :type "PrimitiveComponent Object Reference") (OtherBodyIndex :type Integer) (bFromSweep :type Boolean) (SweepResult :type "HitResult Structure (by ref)"))
  ;[1 1 1] Set In Range if Overlap w/Sphere
  (set `self.InRange` true))

(event `self.ReceiveTick`
  (params (DeltaSeconds :type "Float (single-precision)"))
  ;[1 1 1] Line Trace when within Sphere
  (if (`self.InRange`)
    (bind _asbp_player (cast `/Game/Boo/Player/BP_Player` (`GameplayStatics.GetPlayerCharacter` 0)))
    (bind _firstpersoncameracomponent (`BooCharacter.FirstPersonCameraComponent` _asbp_player))
    (bind _returnvalue (`SceneComponent.K2_GetComponentLocation` _firstpersoncameracomponent))
    (bind _outhit (`KismetSystemLibrary.LineTraceSingle` :`Start` _returnvalue :`End` (+ _returnvalue (* (`KismetMathLibrary.GetForwardVector` (`SceneComponent.K2_GetComponentRotation` _firstpersoncameracomponent)) 5000.0)) :`TraceChannel` "TraceTypeQuery1" :`bIgnoreSelf` false))
    (if (== (`.HitComponent` (`GameplayStatics.BreakHitResult` _outhit)) (`self.Chest`))
      (set `self.inRangeAndHighlighted` true)
      (`MeshComponent.SetVectorParameterValueOnMaterials` (`self.Chest`) "ColorParam" (1.0 0.8 0.0))
      (bind _returnvalue_2 (`|CreateWidget` "/Game/Boo/UI/WBP_Interact.WBP_Interact_C"))
      (if (`self.isLocked`)
        (set `self.ChestMessage` (`KismetStringLibrary.Concat_StrStr` (`KismetStringLibrary.Concat_StrStr` "Locked. Use " (`KismetStringLibrary.ToUpper` (`self.keyToOpen`))) " To Open"))
        (elif (`self.isOpen`)
          (set `self.ChestMessage` (`KismetStringLibrary.Concat_StrStr` "Open. Click to take " (`self.Treasure`)))
          (elif (`self.isEmpty`)
            (set `self.ChestMessage` "Empty")
            (else
              (bind _output_get (set `self.ChestMessage` "Unlocked"))))))
      (`/Game/Boo/UI/WBP_Interact.UpdateText` _returnvalue_2 _output_get)
      (`UserWidget.AddToViewport` _returnvalue_2 0)
      (else
        (set `self.inRangeAndHighlighted` false)
        (`MeshComponent.SetVectorParameterValueOnMaterials` (`self.Chest`) "ColorParam" (0.1 0.05 0.01))
        (bind _foundwidgets (`WidgetBlueprintLibrary.GetAllWidgetsOfClass` "/Game/Boo/UI/WBP_Interact.WBP_Interact_C"))
        (`Widget.RemoveFromParent` _foundwidgets)))))

(event `Event UnlockTheChest`
  (bind _returnvalue (`GameplayStatics.GetPlayerCharacter` 0))
  ;[1 1 1] Unlock The Chest
  (bind _asbp_player (cast `/Game/Boo/Player/BP_Player` _returnvalue))
  (bind _inventory (`/Game/Boo/Player/BP_Player.Inventory` _asbp_player))
  (if (and (`KismetArrayLibrary.Array_Contains` _inventory (`self.keyToOpen`)) (`PrimitiveComponent.IsOverlappingActor` (`self.Sphere`) _returnvalue) (`self.inRangeAndHighlighted`) (!= (`self.isLocked`) false))
    (set `self.isLocked` false)
    (`KismetArrayLibrary.Array_Set` _inventory (`KismetArrayLibrary.Array_Find` _inventory (`self.keyToOpen`)) "EMPTY")
    (bind _foundwidgets (`WidgetBlueprintLibrary.GetAllWidgetsOfClass` "/Game/Boo/UI/WBP_Interact.WBP_Interact_C"))
    (`Widget.RemoveFromParent` _foundwidgets)))

(event `Event OpenTheChest`
  ;[1 1 1] Open Chest if Player In Range, Chest is Highlighted, and Chest is Unlocked
  (if (and (`PrimitiveComponent.IsOverlappingActor` (`self.Sphere`) (`GameplayStatics.GetPlayerCharacter` 0)) (`self.inRangeAndHighlighted`) (!= (`self.isLocked`) true))
    (if (not (`self.isEmpty`))
      (set `self.isOpen` true))
    (`SceneComponent.K2_SetRelativeLocation` (`self.Chest`) (0.0 0.0 50.0) false false)
    (bind _foundwidgets (`WidgetBlueprintLibrary.GetAllWidgetsOfClass` "/Game/Boo/UI/WBP_Interact.WBP_Interact_C"))
    (`Widget.RemoveFromParent` _foundwidgets)))

(event `Event LootTheChest`
  ;[1 1 1] Loot The Chest if Player in Range, Chest is Highlighted, Chest is Open and Contains Loot, and Player has Inventory Space
  (bind _asbp_player (cast `/Game/Boo/Player/BP_Player` (`GameplayStatics.GetPlayerCharacter` 0)))
  (bind _inventory (`/Game/Boo/Player/BP_Player.Inventory` _asbp_player))
  (if (and (`PrimitiveComponent.IsOverlappingActor` (`self.Sphere`) (`GameplayStatics.GetPlayerCharacter` 0)) (`self.inRangeAndHighlighted`) (`self.isOpen`) (`KismetStringLibrary.NotEqual_StrStr` (`self.Treasure`) "EMPTY") (`KismetArrayLibrary.Array_Contains` _inventory "EMPTY"))
    (`KismetArrayLibrary.Array_Set` _inventory (`KismetArrayLibrary.Array_Find` _inventory "EMPTY") (`self.Treasure`))
    (set `self.Treasure` "EMPTY")
    (set `self.isEmpty` true)
    (set `self.isOpen` false)
    (`KismetSystemLibrary.PrintString` "Hello")
    (bind _foundwidgets (`WidgetBlueprintLibrary.GetAllWidgetsOfClass` "/Game/Boo/UI/WBP_Interact.WBP_Interact_C"))
    (`Widget.RemoveFromParent` _foundwidgets)))

(event `self.Sphere.OnComponentEndOverlap`
  (params (OverlappedComponent :type "PrimitiveComponent Object Reference") (OtherActor :type "Actor Object Reference") (OtherComp :type "PrimitiveComponent Object Reference") (OtherBodyIndex :type Integer))
  ;[1 1 1] Resets the Widget upon Exiting Volume
  (set `self.InRange` false)
  (set `self.inRangeAndHighlighted` false)
  (`MeshComponent.SetVectorParameterValueOnMaterials` (`self.Chest`) "ColorParam" (0.1 0.05 0.01))
  (bind _foundwidgets (`WidgetBlueprintLibrary.GetAllWidgetsOfClass` "/Game/Boo/UI/WBP_Interact.WBP_Interact_C"))
  (`Widget.RemoveFromParent` _foundwidgets))

(fn `UserConstructionScript`)