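; BP_Interactable is a configurable world object the player can unlock, open and loot for points.
; When looked at within its overlap volume, it turns yellow and shows a WBP_Interact prompt built from its state, with optional text overrides.
; Interacting moves matching keys from BP_Player's inventory into the locks, attaching key meshes at sockets.
; It then swaps to opened and empty meshes, placing loot in an empty inventory slot.
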(event `self.ReceiveTick`
  (params (DeltaSeconds :type "Float (single-precision)")))

(event `self.ReceiveBeginPlay`
  (bind _messagelineone_override_unlocked (`self.MessageLineOne_Override_Unlocked`))
  (bind _messagelinetwo_override_unlocked (`self.MessageLineTwo_Override_Unlocked`))
  (bind _messagelineone_override_locked (`self.MessageLineOne_Override_Locked`))
  (bind _messagelinetwo_override_locked (`self.MessageLineTwo_Override_Locked`))
  ;[1 1 1] Set Messaging on Start
  (if (`self.isLocked`)
    ;[1 1 1] Locked Messaging
    (if (`KismetStringLibrary.NotEqual_StrStr` _messagelineone_override_locked "DEFAULT")
      (set `self.MessageLineOne` _messagelineone_override_locked)
      (else
        (set `self.MessageLineOne` (`KismetStringLibrary.Concat_StrStr` "LOCKED " (`self.ObjectName`)))))
    (if (`KismetStringLibrary.NotEqual_StrStr` _messagelinetwo_override_locked "DEFAULT")
      (set `self.MessageLineTwo` _messagelinetwo_override_locked)
      (else
        (bind _fullyunlocked (`/Game/Boo/Art/BPFL_Interact.GetRemainingKeys` (`self.KeysToOpen`)))
        (set `self.MessageLineTwo` (`KismetStringLibrary.Concat_StrStr` " USE " (`KismetStringLibrary.JoinStringArray` _fullyunlocked "  ") " TO OPEN"))))
    (else
      ;[1 1 1] Unlocked Messaging
      (set `self.isOpened` true)
      (if (`KismetStringLibrary.NotEqual_StrStr` _messagelineone_override_unlocked "DEFAULT")
        (set `self.MessageLineOne` _messagelineone_override_unlocked)
        (else
          (set `self.MessageLineOne` (`KismetStringLibrary.Concat_StrStr` "UNLOCKED " (`self.ObjectName`)))))
      (if (`KismetStringLibrary.NotEqual_StrStr` _messagelinetwo_override_unlocked "DEFAULT")
        (set `self.MessageLineTwo` _messagelinetwo_override_unlocked)
        (else
          (set `self.MessageLineTwo` "CLICK TO OPEN"))))))

(event `self.ReceiveActorBeginOverlap`
  (params (OtherActor :type "Actor Object Reference"))
  ;[1 1 1] Tell the Player when they are in or out of the Check Volume
  (set `self.inRange` true))

(event `self.ReceiveActorEndOverlap`
  (params (OtherActor :type "Actor Object Reference"))
  ;[1 1 1] Tell the Player when they are in or out of the Check Volume
  (set `self.inRange` false)
  (`self.ResetMaterialsAndWidget`))

(event `/Game/Boo/Player/BPI_Player.StartLookingAt`
  (bind _staticmesh (`self.StaticMesh`))
  ;[1 1 1] When the Object is Being Looked At, Change all Materials in the Mesh to Highlight It, and Create a Widget
  (if (`self.isEmpty`)
    _
    (elif (`self.inRange`)
      (set `self.IsBeingLookedAt` true)
      (for _index (range (+ (`PrimitiveComponent.GetNumMaterials` _staticmesh) 1))
        (`PrimitiveComponent.SetMaterial` _staticmesh _index "/Game/Boo/MaterialLibrary/MI_Color_Yellow.MI_Color_Yellow"))
      (bind _returnvalue (`|CreateWidget` "/Game/Boo/UI/WBP_Interact.WBP_Interact_C"))
      (`/Game/Boo/UI/WBP_Interact.UpdateText` _returnvalue (`self.MessageLineOne`) (`self.MessageLineTwo`))
      (bind _foundwidgets (`WidgetBlueprintLibrary.GetAllWidgetsOfClass` "/Game/Boo/UI/WBP_Interact.WBP_Interact_C"))
      ;[1 1 1] Add The Widget to the Viewport Once
      (if (not (> (`KismetArrayLibrary.Array_Length` _foundwidgets) 1))
        (`UserWidget.AddToViewport` _returnvalue 0)))))

(event `/Game/Boo/Player/BPI_Player.StopLookingAt`
  ;[1 1 1] Destroy the Widget and Reset the Materials when the Object is not being looked At
  (`self.ResetMaterialsAndWidget`))

(event `/Game/Boo/Player/BPI_Player.InteractObject`
  ;[1 1 1] Object Interactions
  (if (and (`self.IsBeingLookedAt`) (`self.inRange`))
    (if (`self.isLocked`)
      (`self.UnlockObject`)
      (if (`self.autoUnlock`)
        (if (`self.isOpened`) :!label _label
          (if (`KismetStringLibrary.EqualEqual_StrStr` (`self.Loot`) "EMPTY")
            (set `self.isEmpty` true)
            (set `self.isReady` false)
            (`/Game/Boo/Art/BPFL_Interact.AwardPoints` (`self.pointsAwarded`))
            (else
              (set `self.isReady` true)
              (set `self.isOpened` false)))
          (`self.OpenObject`)
          (`self.ResetMaterialsAndWidget`)
          (elif (`self.isReady`)
            (`self.CollectLoot`)
            (`self.ResetMaterialsAndWidget`)
            (if (not (`KismetStringLibrary.EqualEqual_StrStr` (`self.Loot`) "EMPTY"))
              (bind _returnvalue (`|CreateWidget` "/Game/Boo/UI/WBP_Pickup.WBP_Pickup_C" null (`self.Loot`)))
              (if (not (`Widget.IsVisible` _returnvalue))
                (`UserWidget.AddToViewport` _returnvalue 0))))))
      (else
        (goto _label)))))

(fn `CollectLoot`
  (bind _emptymesh (`self.EmptyMesh`))
  (set `self.isReady` false)
  (set `self.isEmpty` true)
  ;[1 1 1] Update Mesh to Empty Mesh (if Set)
  (`/Engine/EditorBlueprintResources/StandardMacros.IsValid` _emptymesh
    (:`Is Valid`
      (`StaticMeshComponent.SetStaticMesh` (`self.StaticMesh`) _emptymesh))
    (:`Is Not Valid`
      (`SceneComponent.SetVisibility` (`self.StaticMesh`) false false)
      (`PrimitiveComponent.SetCollisionEnabled` (`self.StaticMesh`) "NoCollision")))
  ;[1 1 1] Empty the Inventory
  (bind _asbp_player (cast `/Game/Boo/Player/BP_Player` (`GameplayStatics.GetPlayerCharacter` 0)))
  (bind _inventory (`/Game/Boo/Player/BP_Player.Inventory` _asbp_player))
  (`KismetArrayLibrary.Array_Set` _inventory (`KismetArrayLibrary.Array_Find` _inventory "EMPTY") (`self.Loot`))
  ;[1 1 1] Award Points
  (`/Game/Boo/Art/BPFL_Interact.AwardPoints` (`self.pointsAwarded`)))

(fn `Debug_RenderText`
  (set `self.Debug_RenderTextString` "")
  (for _array_element (`self.KeysToOpen`)
    (if (`.Inserted_5_D9505B414877E18473789FAE53535287` (break `/Game/Boo/Art/LockAndKey` _array_element))
      (bind _output_get (set `self.Debug_RenderTextString` (`KismetStringLibrary.Concat_StrStr` (`self.Debug_RenderTextString`) (break `/Game/Boo/Art/LockAndKey` _array_element) " YES \n")))
      (else
        (bind _output_get_2 (set `self.Debug_RenderTextString` (`KismetStringLibrary.Concat_StrStr` (`self.Debug_RenderTextString`) (break `/Game/Boo/Art/LockAndKey` _array_element) " NO \n")))))
    (`TextRenderComponent.K2_SetText` (`self.TextRender`) (`KismetTextLibrary.Conv_StringToText` _output_get_2))))

(fn `OpenObject`
  (bind _messagelineone_override_open (`self.MessageLineOne_Override_Open`))
  (bind _openedmesh (`self.OpenedMesh`))
  (bind _messagelinetwo_override_open (`self.MessageLineTwo_Override_Open`))
  ;[1 1 1] Update Mesh to Opened Mesh (if Set) and Update Materials List
  (`/Engine/EditorBlueprintResources/StandardMacros.IsValid` _openedmesh
    (:`Is Valid`
      (`StaticMeshComponent.SetStaticMesh` (`self.StaticMesh`) _openedmesh))
    (:`Is Not Valid`
      _))
  ;[1 1 1] Update Interact Widget
  (bind _foundwidgets (`WidgetBlueprintLibrary.GetAllWidgetsOfClass` "/Game/Boo/UI/WBP_Interact.WBP_Interact_C"))
  (if (`KismetStringLibrary.NotEqual_StrStr` _messagelineone_override_open "DEFAULT")
    (set `self.MessageLineOne` _messagelineone_override_open)
    (else
      (set `self.MessageLineOne` (`self.ObjectName`))))
  (if (`KismetStringLibrary.NotEqual_StrStr` _messagelinetwo_override_open "DEFAULT")
    (set `self.MessageLineTwo` _messagelinetwo_override_open)
    (else
      (set `self.MessageLineTwo` (`KismetStringLibrary.Concat_StrStr` "CLICK TO TAKE " (`self.Loot`)))))
  (`/Game/Boo/UI/WBP_Interact.UpdateText` _foundwidgets (`self.MessageLineOne`) (`self.MessageLineTwo`)))

(fn `ResetMaterialsAndWidget`
  (bind _staticmesh (`self.StaticMesh`))
  (set `self.IsBeingLookedAt` false)
  (for _index (range (+ (`PrimitiveComponent.GetNumMaterials` _staticmesh) 1))
    (`PrimitiveComponent.SetMaterial` _staticmesh _index null))
  (bind _foundwidgets (`WidgetBlueprintLibrary.GetAllWidgetsOfClass` "/Game/Boo/UI/WBP_Interact.WBP_Interact_C"))
  (`Widget.RemoveFromParent` _foundwidgets))

(fn `UnlockObject`
  (bind _messagelineone_override_unlocked (`self.MessageLineOne_Override_Unlocked`))
  (bind _messagelinetwo_override_unlocked (`self.MessageLineTwo_Override_Unlocked`))
  ;[1 1 1] Check the Player Inventory. Does it contain any of the remaining, required Keys?
  (bind _asbp_player (cast `/Game/Boo/Player/BP_Player` (`GameplayStatics.GetPlayerCharacter` 0)))
  (bind _output (`/Game/Boo/Art/BPFL_Interact.GetRequiredKeysFromInventory` (`/Game/Boo/Player/BP_Player.Inventory` _asbp_player) (`self.KeysToOpen`)))
  (if (> (`KismetArrayLibrary.Array_Length` _output) 0)
    ;[1 1 1] If So - Insert Them Into the Door and Remove from Inventory
    (bind _output_2 (`/Game/Boo/Art/BPFL_Interact.AddKeysToObject` _output (`self.KeysToOpen`)))
    (set `self.KeysToOpen` _output_2)
    (`/Game/Boo/Art/BPFL_Interact.RemoveKeysFromInventory` _output)
    (for _array_element _output
      (for _array_element_2 (`self.KeysToOpen`)
        (if (`KismetStringLibrary.EqualEqual_StrStr` _array_element (break `/Game/Boo/Art/LockAndKey` _array_element_2))
          (`/Engine/EditorBlueprintResources/StandardMacros.IsValid` (`.Mesh_8_CD3961D54A79E308E8813F91093243ED` (break `/Game/Boo/Art/LockAndKey` _array_element_2))
            (:`Is Valid`
              (bind _returnvalue_location (`KismetMathLibrary.BreakTransform` (`SceneComponent.GetSocketTransform` (`self.StaticMesh`) (`.Socket_12_A611680748BE15495035659333DF1417` (break `/Game/Boo/Art/LockAndKey` _array_element_2)) "RTS_Actor")))
              (bind _returnvalue (`AddComponent|NODE_AddStaticMeshComponent-1` :`RelativeTransform` (`KismetMathLibrary.MakeTransform` _returnvalue_location)))
              (`StaticMeshComponent.SetStaticMesh` _returnvalue (`.Mesh_8_CD3961D54A79E308E8813F91093243ED` (break `/Game/Boo/Art/LockAndKey` _array_element_2))))))))
    ;[1 1 1] Check if all Keys are Inserted
    (bind _fullyunlocked (`/Game/Boo/Art/BPFL_Interact.AreAllKeysInserted` (`self.KeysToOpen`)))
    (if _fullyunlocked
      ;[1 1 1] If So Unlock Object
      (set `self.isOpened` true)
      (set `self.isLocked` false)
      (bind _foundwidgets (`WidgetBlueprintLibrary.GetAllWidgetsOfClass` "/Game/Boo/UI/WBP_Interact.WBP_Interact_C"))
      (if (`KismetStringLibrary.NotEqual_StrStr` _messagelineone_override_unlocked "DEFAULT")
        (set `self.MessageLineOne` _messagelineone_override_unlocked)
        (else
          (set `self.MessageLineOne` (`KismetStringLibrary.Concat_StrStr` "UNLOCKED " (`self.ObjectName`)))))
      (if (`KismetStringLibrary.NotEqual_StrStr` _messagelinetwo_override_unlocked "DEFAULT")
        (set `self.MessageLineTwo` _messagelinetwo_override_unlocked)
        (else
          (set `self.MessageLineTwo` "CLICK TO OPEN")))
      (`/Game/Boo/UI/WBP_Interact.UpdateText` _foundwidgets (`self.MessageLineOne`) (`self.MessageLineTwo`))
      (else
        ;[1 1 1] If Object Still Locked, Show Keys Remaining
        (bind _foundwidgets_2 (`WidgetBlueprintLibrary.GetAllWidgetsOfClass` "/Game/Boo/UI/WBP_Interact.WBP_Interact_C"))
        (bind _fullyunlocked_2 (`/Game/Boo/Art/BPFL_Interact.GetRemainingKeys` (`self.KeysToOpen`)))
        (bind _output_get (set `self.MessageLineOne` (`KismetStringLibrary.Concat_StrStr` "LOCKED " (`self.ObjectName`))))
        (bind _output_get_2 (set `self.MessageLineTwo` (`KismetStringLibrary.Concat_StrStr` "YOU STILL NEED " (`KismetStringLibrary.JoinStringArray` _fullyunlocked_2) " TO OPEN")))
        (`/Game/Boo/UI/WBP_Interact.UpdateText` _foundwidgets_2 _output_get _output_get_2)))))

(fn `UserConstructionScript`)