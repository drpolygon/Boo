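; Lockable door that the player highlights by looking at it, unlocks with a named inventory key and opens.
; While the player is inside the sphere, Tick traces from the first-person camera, tints the door and creates a status widget every frame it is hit.
; UnlockTheDoor replaces the key with "EMPTY" in the inventory.
; OpenTheDoor snaps the unlocked mesh to a fixed relative location; both events require overlap and highlight.
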(event `self.Sphere.OnComponentBeginOverlap`
  (params (OverlappedComponent :type "PrimitiveComponent Object Reference") (OtherActor :type "Actor Object Reference") (OtherComp :type "PrimitiveComponent Object Reference") (OtherBodyIndex :type Integer) (bFromSweep :type Boolean) (SweepResult :type "HitResult Structure (by ref)"))
  ;[1 1 1] Set In Range if Overlap w/Sphere
  (set `self.InRange` true))

(event `self.ReceiveTick`
  (params (DeltaSeconds :type "Float (single-precision)"))
  ;[1 1 1] Cast Line Trace from Player Camera when In Range
  (if (`self.InRange`)
    (bind _asbp_player (cast `/Game/Boo/Player/BP_Player` (`GameplayStatics.GetPlayerCharacter` 0)))
    (bind _firstpersoncameracomponent (`BooCharacter.FirstPersonCameraComponent` _asbp_player))
    (bind _returnvalue (`SceneComponent.K2_GetComponentLocation` _firstpersoncameracomponent))
    (bind _outhit (`KismetSystemLibrary.LineTraceSingle` :`Start` _returnvalue :`End` (+ _returnvalue (* (`KismetMathLibrary.GetForwardVector` (`SceneComponent.K2_GetComponentRotation` _firstpersoncameracomponent)) 5000.0)) :`TraceChannel` "TraceTypeQuery1" :`bIgnoreSelf` false))
    (if (== (`.HitComponent` (`GameplayStatics.BreakHitResult` _outhit)) (`self.StaticDoor`))
      (set `self.inRangeAndHighlighted` true)
      (`MeshComponent.SetVectorParameterValueOnMaterials` (`self.StaticDoor`) "ColorParam" (1.0 0.8 0.0))
      (bind _returnvalue_2 (`|CreateWidget` "/Game/Boo/UI/WBP_Interact.WBP_Interact_C"))
      (if (`self.isLocked`)
        (bind _output_get (set `self.DoorStatusString` (`KismetStringLibrary.Concat_StrStr` (`KismetStringLibrary.Concat_StrStr` "Locked. Use " (`self.keyToOpen`)) " to Open")))
        (elif (`self.isOpen`)
          (set `self.DoorStatusString` "Open")
          (else
            (set `self.DoorStatusString` "Unlocked"))))
      (`/Game/Boo/UI/WBP_Interact.UpdateText` _returnvalue_2 _output_get)
      (`UserWidget.AddToViewport` _returnvalue_2 0)
      (else
        (set `self.inRangeAndHighlighted` false)
        (`MeshComponent.SetVectorParameterValueOnMaterials` (`self.StaticDoor`) "ColorParam" (0.2 1.0 0.0))
        (bind _foundwidgets (`WidgetBlueprintLibrary.GetAllWidgetsOfClass` "/Game/Boo/UI/WBP_Interact.WBP_Interact_C"))
        (`Widget.RemoveFromParent` _foundwidgets)))))

(event `Event UnlockTheDoor`
  (bind _returnvalue (`GameplayStatics.GetPlayerCharacter` 0))
  (bind _keytoopen (`self.keyToOpen`))
  ;[1 1 1] Unlock The Door
  (bind _asbp_player (cast `/Game/Boo/Player/BP_Player` _returnvalue))
  (bind _inventory (`/Game/Boo/Player/BP_Player.Inventory` _asbp_player))
  (if (and (`KismetArrayLibrary.Array_Contains` _inventory _keytoopen) (`PrimitiveComponent.IsOverlappingActor` (`self.Sphere`) _returnvalue) (`self.inRangeAndHighlighted`) (!= (`self.isLocked`) false))
    (set `self.isLocked` false)
    (`KismetArrayLibrary.Array_Set` _inventory (`KismetArrayLibrary.Array_Find` _inventory _keytoopen) "EMPTY")
    (bind _foundwidgets (`WidgetBlueprintLibrary.GetAllWidgetsOfClass` "/Game/Boo/UI/WBP_Interact.WBP_Interact_C"))
    (`Widget.RemoveFromParent` _foundwidgets)))

(event `Event OpenTheDoor`
  ;[1 1 1] Open Door if Player In Range, Door is Highlighted, and Door is Unlocked
  (if (and (`PrimitiveComponent.IsOverlappingActor` (`self.Sphere`) (`GameplayStatics.GetPlayerCharacter` 0)) (`self.inRangeAndHighlighted`) (!= (`self.isLocked`) true))
    (set `self.isOpen` true)
    (`SceneComponent.K2_SetRelativeLocation` (`self.StaticDoor`) (-60.0 0.0 200.0) false false)
    (bind _foundwidgets (`WidgetBlueprintLibrary.GetAllWidgetsOfClass` "/Game/Boo/UI/WBP_Interact.WBP_Interact_C"))
    (`Widget.RemoveFromParent` _foundwidgets)))

(event `self.Sphere.OnComponentEndOverlap`
  (params (OverlappedComponent :type "PrimitiveComponent Object Reference") (OtherActor :type "Actor Object Reference") (OtherComp :type "PrimitiveComponent Object Reference") (OtherBodyIndex :type Integer))
  ;[1 1 1] Resets the Widget upon Exiting Volume
  (set `self.InRange` false)
  (set `self.inRangeAndHighlighted` false)
  (`MeshComponent.SetVectorParameterValueOnMaterials` (`self.StaticDoor`) "ColorParam" (0.2 1.0 0.0))
  (bind _foundwidgets (`WidgetBlueprintLibrary.GetAllWidgetsOfClass` "/Game/Boo/UI/WBP_Interact.WBP_Interact_C"))
  (`Widget.RemoveFromParent` _foundwidgets))

(fn `UserConstructionScript`)