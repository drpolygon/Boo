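; BP_Pickup is an interactable item that the player can look at and collect into their inventory.
; Overlap begin and end toggle the player's IsInCheckVolume flag.
; Being looked at swaps all mesh materials to yellow and shows a WBP_Interact prompt; looking away restores cached materials and removes the prompt.
; Interacting while looked at writes the item into the first "EMPTY" inventory slot, then destroys the actor.
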(event `self.ReceiveBeginPlay`
  (bind _staticmesh (`self.StaticMesh`))
  (bind _materialslist (`self.MaterialsList`))
  (for _index (range (+ (`PrimitiveComponent.GetNumMaterials` _staticmesh) 1))
    (`KismetArrayLibrary.Array_Add` _materialslist (`PrimitiveComponent.GetMaterial` _staticmesh _index)))
  (for _ _materialslist
    _))

(event `self.ReceiveActorBeginOverlap`
  (params (OtherActor :type "Actor Object Reference"))
  (bind _asbp_player (cast `/Game/Boo/Player/BP_Player` (`GameplayStatics.GetPlayerCharacter` 0)))
  (set `/Game/Boo/Player/BP_Player.isInCheckVolume` true _asbp_player))

(event `self.ReceiveActorEndOverlap`
  (params (OtherActor :type "Actor Object Reference"))
  (bind _asbp_player (cast `/Game/Boo/Player/BP_Player` (`GameplayStatics.GetPlayerCharacter` 0)))
  (set `/Game/Boo/Player/BP_Player.isInCheckVolume` false _asbp_player))

(event `/Game/Boo/Player/BPI_Player.StartLookingAt`
  (set `self.IsBeingLookedAt` true)
  (for (_ _array_index) (`self.MaterialsList`)
    (`PrimitiveComponent.SetMaterial` (`self.StaticMesh`) _array_index "/Game/Boo/MaterialLibrary/MI_Color_Yellow.MI_Color_Yellow"))
  (bind _returnvalue (`|CreateWidget` "/Game/Boo/UI/WBP_Interact.WBP_Interact_C"))
  (`/Game/Boo/UI/WBP_Interact.UpdateText` _returnvalue (`self.Object`))
  (`/Engine/EditorBlueprintResources/StandardMacros.DoOnce` false :!label _label
    (:`Completed`
      (`UserWidget.AddToViewport` _returnvalue 0))))

(event `/Game/Boo/Player/BPI_Player.StopLookingAt`
  (set `self.IsBeingLookedAt` false)
  (for (_array_element _array_index) (`self.MaterialsList`)
    (`PrimitiveComponent.SetMaterial` (`self.StaticMesh`) _array_index _array_element))
  (bind _foundwidgets (`WidgetBlueprintLibrary.GetAllWidgetsOfClass` "/Game/Boo/UI/WBP_Interact.WBP_Interact_C"))
  (`Widget.RemoveFromParent` _foundwidgets)
  (goto _label :!via `Reset`))

(event `/Game/Boo/Player/BPI_Player.InteractObject`
  (if (`self.IsBeingLookedAt`)
    (bind _asbp_player (cast `/Game/Boo/Player/BP_Player` (`GameplayStatics.GetPlayerCharacter` 0)))
    (bind _inventory (`/Game/Boo/Player/BP_Player.Inventory` _asbp_player))
    (`KismetArrayLibrary.Array_Set` _inventory (`KismetArrayLibrary.Array_Find` _inventory "EMPTY") (`self.Object`))
    (`self.K2_DestroyActor`)))

(fn `UserConstructionScript`)