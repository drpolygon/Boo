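; First-person player character that handles sprinting, creates the inventory HUD and interacts with objects inside check volumes.
; While IsInCheckVolume is set, Tick line-traces from the camera and sends look-at start or stop messages to a cached BPI_Player actor.
; Interact messages that cached actor, which is never cleared.
; An author comment flags warnings when crossing volumes as actors are destroyed.
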(event `InputAction|Sprint`
  (params (Key :type "Key Structure" :default "AnyKey"))
  ;[1 1 1] Sprinting
  (:`Pressed`
    (set `CharacterMovementComponent.MaxWalkSpeed` 1500.0 (`self.CharacterMovement`)))
  (:`Released`
    (set `CharacterMovementComponent.MaxWalkSpeed` 600.0 (`self.CharacterMovement`))))

(event `self.ReceiveBeginPlay`
  ;[1 1 1] HUD: Inventory
  (bind _returnvalue (`|CreateWidget` "/Game/Boo/UI/WBP_Inventory.WBP_Inventory_C"))
  (`UserWidget.AddToViewport` _returnvalue 0))

(event `self.ReceiveTick`
  (params (DeltaSeconds :type "Float (single-precision)"))
  (bind _firstpersoncameracomponent (`self.FirstPersonCameraComponent`))
  (bind _returnvalue (`SceneComponent.K2_GetComponentLocation` _firstpersoncameracomponent))
  (if (`self.isInCheckVolume`)
    (bind (_outhit _returnvalue_2) (`KismetSystemLibrary.LineTraceSingle` _returnvalue (+ _returnvalue (* (`KismetMathLibrary.GetForwardVector` (`SceneComponent.K2_GetComponentRotation` _firstpersoncameracomponent)) 5000.0)) "TraceTypeQuery1"))
    (if _returnvalue_2
      (bind (_bblockinghit _binitialoverlap _time _location _impactpoint _normal _impactnormal _physmat _hitactor) (`GameplayStatics.BreakHitResult` _outhit))
      (bind _output_get (set `self.CurrentHitActor` _hitactor))
      (if (`KismetSystemLibrary.DoesImplementInterface` _hitactor "/Game/Boo/Player/BPI_Player.BPI_Player_C")
        (bind _output_get_2 (set `self.ValidHitActor` _output_get))
        (message `/Game/Boo/Player/BPI_Player.StartLookingAt` _output_get_2)
        (else
          ;[1 0 0] BUG HERE - Going in and out of volume while actor is being destroyed causes warnings
          (message `/Game/Boo/Player/BPI_Player.StopLookingAt` (`self.ValidHitActor`) :!label _label)))
      (else
        (goto _label)))))

(event `InputAction|Interact`
  (params (Key :type "Key Structure" :default "AnyKey"))
  (:`Pressed`
    (if (`self.isInCheckVolume`)
      (message `/Game/Boo/Player/BPI_Player.InteractObject` (`self.ValidHitActor`)))))

(fn `UserConstructionScript`)